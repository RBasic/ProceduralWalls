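; Spline wall actor that builds a row of spline meshes along an editable, optionally closed spline in its Construction Script.
; It clears near-zero-size meshes, bubble-sorts the rest largest first by bounding-box or fixed size on the chosen axis, then greedily places the largest that fits.
; When none fits, a final mesh is deformed to close the gap to the spline's end, or start if looped.
; Tangents are clamped to mesh size.
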(event EventBeginPlay)

(event Collision|EventActorBeginOverlap
  (params (OtherActor :type Actor%20Object%20Reference)))

(event EventTick
  (params (DeltaSeconds :type Float%20%28single-precision%29)))

(fn ConstructionScript
  (bind _tabmeshes (Variables|Default|GetTabMeshes))
  (bind _spline (Variables|Default|GetSpline))
  (bind _enumaxe (Variables|Default|GetEnumAxe))
  (Spline|SetClosedLoop (Variables|Default|GetSpline) (Variables|Default|GetClosedLoop?) true)
  ;[1 1 1] Prepare meshes array/spline
  (if (and (> (Utilities|Array|Length _tabmeshes) 0) (Utilities|IsValid (Utilities|Array|Get(acopy) _tabmeshes)))
    (CallFunction|CheckMeshSize _enumaxe)
    (CallFunction|SortTab _enumaxe)
    (LocalVariables|SetSplineDist (Spline|GetSplineLength (Variables|Default|GetSpline)))
    (while (and (< (LocalVariables|GetActualDist) (LocalVariables|GetSplineDist)) (LocalVariables|GetCanPutWall?))
      (LocalVariables|SetCanPutWall? false)
      (LocalVariables|SetStartLocation (.LocationDistance (CallFunction|SplineInfos (LocalVariables|GetActualDist))))
      (LocalVariables|SetStartTangent (.TangentDistance (CallFunction|SplineInfos (LocalVariables|GetActualDist))))
      (LocalVariables|SetIndex 0)
      ;[1 1 1] SearchBestMesh
      (bind (_array_element _array_index) (Utilities|Array|ForEachLoopwithBreak (Variables|Default|GetTabMeshes) :!label _label)
        (:LoopBody
          (Utilities|IsValid _array_element
            (:Is%20Valid
              (LocalVariables|SetIndex _array_index)
              (if (>= (LocalVariables|GetSplineDist) (+ (CallFunction|GetMeshSize _array_element (Variables|Default|GetEnumAxe)) (LocalVariables|GetActualDist)))
                (LocalVariables|SetActualDist (+ (CallFunction|GetMeshSize _array_element (Variables|Default|GetEnumAxe)) (LocalVariables|GetActualDist)))
                (LocalVariables|SetCanPutWall? true)
                (goto _label Break)))))
        (:Completed
          ;[1 1 1] Place Mesh With Spline Tangent
          (LocalVariables|SetEndLocation (Math|Vector|SelectVector (.LocationDistance (CallFunction|SplineInfos (LocalVariables|GetActualDist) (select (Class|SplineComponent|IsClosedLoop _spline) 0 (- (Spline|GetNumberOfSplinePoints _spline) 1)))) (.LocationPoint (CallFunction|SplineInfos (LocalVariables|GetActualDist) (select (Class|SplineComponent|IsClosedLoop _spline) 0 (- (Spline|GetNumberOfSplinePoints _spline) 1)))) (LocalVariables|GetCanPutWall?)))
          (LocalVariables|SetEndTangent (Math|Vector|SelectVector (.TangentDistance (CallFunction|SplineInfos (LocalVariables|GetActualDist) (select (Class|SplineComponent|IsClosedLoop _spline) 0 (- (Spline|GetNumberOfSplinePoints _spline) 1)))) (.TangentPoint (CallFunction|SplineInfos (LocalVariables|GetActualDist) (select (Class|SplineComponent|IsClosedLoop _spline) 0 (- (Spline|GetNumberOfSplinePoints _spline) 1)))) (LocalVariables|GetCanPutWall?)))
          (bind _returnvalue (AddComponent|AddSplineMeshComponent false))
          (Components|StaticMesh|SetStaticMesh _returnvalue (Utilities|Array|Get(acopy) (Variables|Default|GetTabMeshes) (LocalVariables|GetIndex)))
          (SplineMesh|SetForwardAxis _returnvalue (Variables|Default|GetEnumAxe) true)
          (SplineMesh|SetStartandEnd _returnvalue (LocalVariables|GetStartLocation) (Math|Vector|ClampVectorSize (LocalVariables|GetStartTangent) 0.0 (CallFunction|GetMeshSize (Utilities|Array|Get(acopy) (Variables|Default|GetTabMeshes) (LocalVariables|GetIndex)) (Variables|Default|GetEnumAxe))) (LocalVariables|GetEndLocation) (Math|Vector|ClampVectorSize (LocalVariables|GetEndTangent) 0.0 (CallFunction|GetMeshSize (Utilities|Array|Get(acopy) (Variables|Default|GetTabMeshes) (LocalVariables|GetIndex)) (Variables|Default|GetEnumAxe))) true :!class /Script/Engine.SplineMeshComponent))))))

(fn GetMeshSize
  (params (Target :type Static%20Mesh%20Object%20Reference) (Axe :type ESplineMeshAxis%20Enum :default "X"))
  (bind _returnvalue (StaticMesh|GetBoundingBox Target))
  (return (select (Variables|Default|GetUsingBoundingBox?) (+ (Math|Float|Absolute(Float) (Utilities|Select :Index Axe :X (.x (.min _returnvalue)) :Y (.y (.min _returnvalue)) :Z (.z (.min _returnvalue)))) (Math|Float|Absolute(Float) (Utilities|Select :Index Axe :X (.x (.max _returnvalue)) :Y (.y (.max _returnvalue)) :Z (.z (.max _returnvalue))))) (Variables|Default|GetMeshSize))))

(fn SplineInfos
  (params (Distance :type Float%20%28double-precision%29) (PointIndex :type Integer))
  (bind _spline (Variables|Default|GetSpline))
  (return (Spline|GetLocationatSplinePoint _spline PointIndex "Local") (Spline|GetTangentatSplinePoint _spline PointIndex "Local") (Spline|GetLocationatDistanceAlongSpline _spline Distance "Local") (Spline|GetTangentatDistanceAlongSpline _spline Distance "Local")))

(fn SortTab
  (params (Axe :type ESplineMeshAxis%20Enum :default "X"))
  (bind _index (Utilities|ForLoopAdvanced (Utilities|Array|LastIndex (Variables|Default|GetTabMeshes)) 1 1)
    (:LoopBody
      (LocalVariables|Seti _index)
      (LocalVariables|SetSorted? true)
      (for _index_2 (range 0 (- (LocalVariables|Geti) 1))
        (LocalVariables|Setj _index_2)
        (if (> (CallFunction|GetMeshSize (Utilities|Array|Get(acopy) (Variables|Default|GetTabMeshes) (+ (LocalVariables|Getj) 1)) Axe) (CallFunction|GetMeshSize (Utilities|Array|Get(acopy) (Variables|Default|GetTabMeshes) (LocalVariables|Getj)) Axe))
          (Utilities|Array|Swap (Variables|Default|GetTabMeshes) (LocalVariables|Getj) (+ (LocalVariables|Getj) 1))
          (LocalVariables|SetSorted? false)))
      (if (LocalVariables|GetSorted?)
        (return)))
    (:Completed
      (return))))

(fn CheckMeshSize
  (params (Axe :type ESplineMeshAxis%20Enum :default "X"))
  (for (_array_element _array_index) (Variables|Default|GetTabMeshes)
    (if (and (<= (CallFunction|GetMeshSize _array_element Axe) 1.0) (Utilities|IsValid _array_element))
      (Utilities|Array|SetArrayElem (Variables|Default|GetTabMeshes) _array_index 0)))
  (return))